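; Monster eye actor that blinks and turns to follow the player inside its detection cone.
; A looping delay and FlipFlop alternately play and reverse a timeline that rotates both eyelids every 1.5 seconds.
; Cone overlap runs a timeline as a tick, smoothly rotating the eye within socket-relative clamped limits and firing debug-drawn Pawn traces, whose results are unused.
; The construction script derives trace length from a marker component.
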(event `self.ReceiveBeginPlay`
  (`/Engine/EditorBlueprintResources/StandardMacros.FlipFlop` :!label _label
    (:`A`
      (`self.ToggleEyes` true))
    (:`B`
      (`self.ToggleEyes` false)))
  (`KismetSystemLibrary.Delay` 1.5)
  (goto _label))

(event `ToggleEyes`
  (params (`Close?` :type Boolean))
  (if `Close?`
    (bind (_direction _alpha) (`Timeline|RotateEyeLids` :!via `PlayFromStart` :!label _label_2)
      (:`Update`
        (`SceneComponent.K2_SetRelativeRotation` (`self.TopEyeLid`) (`KismetMathLibrary.RLerp` (struct :`Pitch` 45.0) (struct) _alpha) false false)
        (`SceneComponent.K2_SetRelativeRotation` (`self.BottomEyeLid`) (`KismetMathLibrary.RLerp` (struct :`Pitch` -45.0) (struct) _alpha) false false)))
    (else
      (goto _label_2 :!via `ReverseFromEnd`))))

(event `self.Cone.OnComponentBeginOverlap`
  (params (OverlappedComponent :type "PrimitiveComponent Object Reference") (OtherActor :type "Actor Object Reference") (OtherComp :type "PrimitiveComponent Object Reference") (OtherBodyIndex :type Integer) (bFromSweep :type Boolean) (SweepResult :type "HitResult Structure (by ref)"))
  (bind _pursueclampz (`self.PursueClampZ`))
  (bind _eye (`self.Eye`))
  (bind _pursueclampz_2 (`self.PursueClampZ`))
  (bind _returnvalue (`SceneComponent.K2_GetComponentLocation` (`self.Cone`)))
  (bind (_returnvalue_roll _returnvalue_pitch _returnvalue_yaw) (`KismetMathLibrary.BreakRotator` (`KismetMathLibrary.InverseTransformRotation` (`SceneComponent.K2_GetComponentToWorld` (`self.EyeSocket`)) (`KismetMathLibrary.FindLookAtRotation` (`SceneComponent.K2_GetComponentLocation` _eye) (`self.K2_GetActorLocation` (`GameplayStatics.GetPlayerPawn` 0))))))
  (if (== OtherActor (`GameplayStatics.GetPlayerPawn` 0))
    (`Timeline|SendRayCast` :!label _label_3
      (:`Update`
        (`|ExecutionSequence`
          (:`then_0`
            (`KismetSystemLibrary.LineTraceSingleForObjects` :`Start` _returnvalue :`End` (+ _returnvalue (* (`KismetMathLibrary.Conv_RotatorToVector` (`KismetMathLibrary.FindLookAtRotation` _returnvalue (`SceneComponent.K2_GetComponentLocation` (`Actor.RootComponent` (`GameplayStatics.GetPlayerPawn` 0))))) (`self.TraceLength`))) :`ObjectTypes` (`|MakeArray` "ObjectTypeQuery3" :!type "EObjectTypeQuery Enum") :`DrawDebugType` "Persistent" :`DrawTime` 2.0))
          (:`then_1`
            (`SceneComponent.K2_SetRelativeRotation` _eye (`KismetMathLibrary.RLerp` (`SceneComponent.RelativeRotation` _eye) (`KismetMathLibrary.MakeRotator` _returnvalue_roll (`KismetMathLibrary.FClamp` _returnvalue_pitch (* _pursueclampz -1.0) _pursueclampz) (`KismetMathLibrary.FClamp` _returnvalue_yaw (* _pursueclampz_2 -1.0) _pursueclampz_2)) (* (`GameplayStatics.GetWorldDeltaSeconds`) (`self.RotateSpeed`)) true) false false)))))))

(event `self.Cone.OnComponentEndOverlap`
  (params (OverlappedComponent :type "PrimitiveComponent Object Reference") (OtherActor :type "Actor Object Reference") (OtherComp :type "PrimitiveComponent Object Reference") (OtherBodyIndex :type Integer))
  (if (== OtherActor (`GameplayStatics.GetPlayerPawn` 0))
    (goto _label_3 :!via `Stop`)))

(fn `UserConstructionScript`
  (`TimelineComponent.SetPlayRate` (`self.RotateEyeLids`) 2.0)
  (set `self.TraceLength` (`KismetMathLibrary.VSize` (- (`SceneComponent.K2_GetComponentLocation` (`self.RayCastLength`)) (`SceneComponent.K2_GetComponentLocation` (`self.Cone`))))))