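; Monster eye sensor that spots the player and reports sight gained or lost to its AssignedMonster.
; Player overlap with the vision cone starts a timeline that repeatedly line-traces for line of sight.
; If CanClose, eyelids blink at random intervals unless the blackboard TargetActor is set, disabling cone collision while shut.
; PursueTarget smoothly turns the eye toward the player, clamped relative to its socket.
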(event `self.ReceiveBeginPlay`
  (`TimelineComponent.SetPlayRate` (`self.RotateEyeLids`) 7.0)
  (if (`self.CanClose`)
    (`KismetSystemLibrary.Delay` (`self.CalculateTimeBeforeClose`) :!label _label)
    (if (!= (`BlackboardComponent.GetValueAsObject` (`AIBlueprintHelperLibrary.GetBlackboard` (`AIBlueprintHelperLibrary.GetAIController` self)) "TargetActor") null)
      (goto _label)
      (else
        (`self.ToggleEyes` true)
        (`KismetSystemLibrary.Delay` (`self.CalculateTimeBeforeOpen`))
        (`self.ToggleEyes` false)
        (goto _label)))))

(event `ToggleEyes`
  (params (`Close?` :type Boolean))
  (bind _cone (`self.Cone`))
  (if `Close?`
    (bind (_direction _alpha) (`Timeline|RotateEyeLids` :!via `PlayFromStart` :!label _label_2)
      (:`Update`
        (`SceneComponent.K2_SetRelativeRotation` (`self.TopEyeLid`) (`KismetMathLibrary.RLerp` (struct :`Pitch` 45.0) (struct) _alpha) false false)
        (`SceneComponent.K2_SetRelativeRotation` (`self.BottomEyeLid`) (`KismetMathLibrary.RLerp` (struct :`Pitch` -45.0) (struct) _alpha) false false))
      (:`Finished`
        (switch `ETimelineDirection` _direction
          (:`Forward`
            (`PrimitiveComponent.SetCollisionEnabled` _cone "NoCollision"))
          (:`Backward`
            (`PrimitiveComponent.SetCollisionEnabled` _cone "QueryOnly")))))
    (else
      (goto _label_2 :!via `ReverseFromEnd`))))

(event `self.Cone.OnComponentBeginOverlap`
  (params (OverlappedComponent :type "PrimitiveComponent Object Reference") (OtherActor :type "Actor Object Reference") (OtherComp :type "PrimitiveComponent Object Reference") (OtherBodyIndex :type Integer) (bFromSweep :type Boolean) (SweepResult :type "HitResult Structure (by ref)"))
  (bind _assignedmonster (`self.AssignedMonster`))
  (bind _victim (`self.Victim`))
  (bind _canseeplayer (`self.CanSeePlayer`))
  (bind _returnvalue (`SceneComponent.K2_GetComponentLocation` (`self.Eye`)))
  (if (== OtherActor (`GameplayStatics.GetPlayerPawn` 0))
    (`|ExecutionSequence`
      (:`then_0`
        (`Timeline|SendRayCast` :!label _label_3
          (:`Update`
            (bind _outhit (`KismetSystemLibrary.LineTraceSingleForObjects` _returnvalue (+ _returnvalue (* (`KismetMathLibrary.Conv_RotatorToVector` (`KismetMathLibrary.FindLookAtRotation` _returnvalue (`self.K2_GetActorLocation` (`self.Victim`)))) (`self.TraceLength`))) (`|MakeArray` "ObjectTypeQuery1" "ObjectTypeQuery3" :!type "EObjectTypeQuery Enum") false (`|MakeArray` (`self.AssignedMonster`)) "None" true (struct :`R` 1.0 :`A` 1.0) (struct :`G` 1.0 :`A` 1.0) 2.0))
            (if (== (`self.Victim`) (`.HitActor` (`GameplayStatics.BreakHitResult` _outhit)))
              (if (not _canseeplayer)
                (set `self.CanSeePlayer` true)
                (`/Game/FirstPersonCPP/Blueprints/MonsterEnemy/BP_Enemy.ReportFromEye` _assignedmonster true _victim))
              (elif _canseeplayer
                (set `self.CanSeePlayer` false)
                (`/Game/FirstPersonCPP/Blueprints/MonsterEnemy/BP_Enemy.ReportFromEye` _assignedmonster false _victim))))))
      (:`then_1`
        (set `self.Victim` OtherActor)))))

(event `self.Cone.OnComponentEndOverlap`
  (params (OverlappedComponent :type "PrimitiveComponent Object Reference") (OtherActor :type "Actor Object Reference") (OtherComp :type "PrimitiveComponent Object Reference") (OtherBodyIndex :type Integer))
  (bind _victim (`self.Victim`))
  (if (== OtherActor _victim)
    (set `self.CanSeePlayer` false)
    (`/Game/FirstPersonCPP/Blueprints/MonsterEnemy/BP_Enemy.ReportFromEye` (`self.AssignedMonster`) false _victim)
    (goto _label_3 :!via `Stop`)))

(event `PursueTarget`
  (`SceneComponent.K2_SetRelativeRotation` (`self.Eye`) (`self.RelativeLookAt`) false false))

(fn `CalculateTimeBeforeClose`
  (returns (Delay :type "Float (double-precision)"))
  (return (`KismetMathLibrary.RandomFloatInRange` (`self.MinTimeBeforeClose`) (`self.MaxTimeBeforeClose`))))

(fn `CalculateTimeBeforeOpen`
  (returns (Delay :type "Float (double-precision)"))
  (return (`KismetMathLibrary.RandomFloatInRange` (`self.MinTimeBeforeOpen`) (`self.MaxTimeBeforeOpen`))))

(fn `RelativeLookAt`
  (returns (ReturnValue :type "Rotator Structure"))
  (bind _pursueclampz (`self.PursueClampZ`))
  (bind _eye (`self.Eye`))
  (bind _pursueclampz_2 (`self.PursueClampZ`))
  (bind (_returnvalue_roll _returnvalue_pitch _returnvalue_yaw) (`KismetMathLibrary.BreakRotator` (`KismetMathLibrary.InverseTransformRotation` (`SceneComponent.K2_GetComponentToWorld` (`self.EyeSocket`)) (`KismetMathLibrary.FindLookAtRotation` (`SceneComponent.K2_GetComponentLocation` _eye) (`self.K2_GetActorLocation` (`GameplayStatics.GetPlayerPawn` 0))))))
  (return (`KismetMathLibrary.RLerp` (`SceneComponent.RelativeRotation` _eye) (`KismetMathLibrary.MakeRotator` _returnvalue_roll (`KismetMathLibrary.FClamp` _returnvalue_pitch (* _pursueclampz -1.0) _pursueclampz) (`KismetMathLibrary.FClamp` _returnvalue_yaw (* _pursueclampz_2 -1.0) _pursueclampz_2)) (* (`GameplayStatics.GetWorldDeltaSeconds`) (`self.RotateSpeed`)) true)))

(fn `UserConstructionScript`
  (`TimelineComponent.SetPlayRate` (`self.RotateEyeLids`) 2.0)
  (set `self.TraceLength` (`KismetMathLibrary.VSize` (- (`SceneComponent.K2_GetComponentLocation` (`self.RayCastLength`)) (`SceneComponent.K2_GetComponentLocation` (`self.Cone`))))))