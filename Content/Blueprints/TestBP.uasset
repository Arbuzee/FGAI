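; Test actor that turns its StaticMesh toward TargetRot at a constant overall rate set by Speed.
; Each Tick interpolates relative pitch and yaw with FInterpToConstant and forces roll to zero.
; Each axis gets a share of Speed proportional to its share of the summed absolute rotation delta, which keeps the two axes in step.
; An earlier yaw-to-pitch ratio version remains unconnected.
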(event `self.ReceiveTick`
  (params (DeltaSeconds :type "Float (single-precision)"))
  (bind _targetrot (`self.TargetRot`))
  (bind _relativerotation (`SceneComponent.RelativeRotation` (`self.StaticMesh`)))
  (bind _returnvalue (`KismetMathLibrary.Abs` (.yaw (`KismetMathLibrary.NormalizedDeltaRotator` _targetrot _relativerotation))))
  (bind _returnvalue_2 (`KismetMathLibrary.Abs` (.pitch (`KismetMathLibrary.NormalizedDeltaRotator` _targetrot _relativerotation))))
  (bind _returnvalue_3 (/ (+ (`KismetMathLibrary.Abs` (.roll (`KismetMathLibrary.NormalizedDeltaRotator` _targetrot _relativerotation))) _returnvalue_2 _returnvalue) (`self.Speed`)))
  (`SceneComponent.K2_SetRelativeRotation` (`self.StaticMesh`) (`KismetMathLibrary.MakeRotator` 0.0 (`KismetMathLibrary.FInterpTo_Constant` (.pitch _relativerotation) (.pitch _targetrot) DeltaSeconds (/ _returnvalue_2 _returnvalue_3)) (`KismetMathLibrary.FInterpTo_Constant` (.yaw _relativerotation) (.yaw _targetrot) DeltaSeconds (/ _returnvalue _returnvalue_3))) false false))

(fn `UserConstructionScript`)